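; Act 1 game state that handles the level's win and death outcomes, caching the player and game instance on BeginPlay.
; Tick polls the game time subsystem and triggers WinGame once when max time is reached, running timed white-screen fades before the loading screen and win save.
; EndGame, when Death is set, fires the player's jumpscare and loads the main menu once through the game instance.
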(event `self.ReceiveBeginPlay`
  (bind _asbp_player (cast `/Game/Blueprints/Act-1/Player/BP_Player` (`GameplayStatics.GetPlayerPawn` 0)))
  (set `self.Player` _asbp_player)
  (bind _asbp_game_info_instance (cast `/Game/Blueprints/AllLevels/BP_GameInfoInstance` (`GameplayStatics.GetGameInstance`)))
  (set `self.GameInstance` _asbp_game_info_instance))

(event `self.ReceiveTick`
  (params (DeltaSeconds :type "Float (single-precision)"))
  (if (`GameTimeSubsystem.ItsMaxTime` (subsystem `GameTimeSubsystem`))
    (`/Engine/EditorBlueprintResources/StandardMacros.DoOnce` false
      (:`Completed`
        (`self.WinGame`)))))

(event `EndGame`
  (if (`self.Death`)
    (`/Game/Blueprints/Act-1/Player/BP_Player.OnJumpscare` (`self.Player`))
    (`/Engine/EditorBlueprintResources/StandardMacros.DoOnce` false
      (:`Completed`
        (`/Game/Blueprints/AllLevels/BP_GameInfoInstance.LoadLevel` (`self.GameInstance`) "/Game/Levels/MainMenu.MainMenu")))))

(event `WinGame`
  (bind _gameinstance (`self.GameInstance`))
  (bind _wb_whitescreen (`/Game/Blueprints/AllLevels/BP_GameInfoInstance.WB_WhiteScreen` _gameinstance))
  (`WidgetLayoutLibrary.RemoveAllWidgets`)
  (`KismetSystemLibrary.CollectGarbage`)
  (`/Game/Blueprints/AllLevels/BP_GameInfoInstance.ShowWhiteScreen` _gameinstance)
  (`/Game/Blueprints/LoadingScreen/Widgets/WB_WhiteTransition.OnFadeIn` _wb_whitescreen)
  (`KismetSystemLibrary.Delay` 1.0)
  (`/Game/Blueprints/AllLevels/BP_GameInfoInstance.FadeIn` (`self.GameInstance`))
  (`KismetSystemLibrary.Delay` 1.0)
  (`/Game/Blueprints/LoadingScreen/Widgets/WB_WhiteTransition.OnFadeOut` _wb_whitescreen)
  (`KismetSystemLibrary.Delay` 1.0)
  (`Widget.RemoveFromParent` _wb_whitescreen)
  (`/Game/Blueprints/AllLevels/BP_GameInfoInstance.ShowLoadingScreen` (`self.GameInstance`))
  (`KismetSystemLibrary.Delay` 0.5)
  (`/Game/Blueprints/AllLevels/BP_GameInfoInstance.WinSaveGame` (`self.GameInstance`)))

(fn `UserConstructionScript`)