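; Act 1 game state that arbitrates monster attacks and handles losing, winning and light-switch events.
; Attack requests fire immediately when the queue is empty and attacks are allowed, otherwise they are inserted into a list by monster-type priority.
; Removing a queue entry blocks attacks, then releases the next after a base plus random delay.
; Death triggers the player's jumpscare, while winning runs timed white-screen fades, loading and a save.
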(event `self.ReceiveBeginPlay`
  (bind _asbp_act_1player (cast `/Game/Blueprints/Act-1/Player/BP_Act-1Player` (`GameplayStatics.GetPlayerPawn` 0)))
  (set `self.Player` _asbp_act_1player)
  (bind _asbp_game_info_instance (cast `/Game/Blueprints/SaveSystem/BP_GameInfoInstance` (`GameplayStatics.GetGameInstance`)))
  (set `self.GameInstance` _asbp_game_info_instance)
  (set `self.CanAllowAttack` true))

(event `EndGame`
  (if (`self.Death`)
    (`/Game/Blueprints/Act-1/Player/BP_Act-1Player.OnJumpscare` (`self.Player`))
    (`/Engine/EditorBlueprintResources/StandardMacros.DoOnce` false
      (:`Completed`
        (`/Game/Blueprints/SaveSystem/BP_GameInfoInstance.LoadLevel` (`self.GameInstance`) "/Game/Levels/MainMenu.MainMenu")))))

(event `WinGame`
  (bind _gameinstance (`self.GameInstance`))
  (bind _wb_whitescreen (`/Game/Blueprints/SaveSystem/BP_GameInfoInstance.WB_WhiteScreen` _gameinstance))
  (`WidgetLayoutLibrary.RemoveAllWidgets`)
  (`KismetSystemLibrary.CollectGarbage`)
  (`/Game/Blueprints/SaveSystem/BP_GameInfoInstance.ShowWhiteScreen` _gameinstance)
  (`/Game/Blueprints/Menu/UI/LoadingScreen/WBP_WhiteTransition.OnFadeIn` _wb_whitescreen)
  (`KismetSystemLibrary.Delay` 1.0)
  (`/Game/Blueprints/SaveSystem/BP_GameInfoInstance.FadeIn` (`self.GameInstance`))
  (`KismetSystemLibrary.Delay` 1.0)
  (`/Game/Blueprints/Menu/UI/LoadingScreen/WBP_WhiteTransition.OnFadeOut` _wb_whitescreen)
  (`KismetSystemLibrary.Delay` 1.0)
  (`Widget.RemoveFromParent` _wb_whitescreen)
  (`/Game/Blueprints/SaveSystem/BP_GameInfoInstance.ShowLoadingScreen` (`self.GameInstance`))
  (`KismetSystemLibrary.Delay` 0.5)
  (`/Game/Blueprints/SaveSystem/BP_GameInfoInstance.WinSaveGame` (`self.GameInstance`)))

(event `SwitchLights`
  (`self.DarknessChange`))

(event `RemoveMonsterFromQueue`
  (set `self.CanAllowAttack` false)
  (`KismetArrayLibrary.Array_Remove` (`self.MonstersAttackList`))
  (if (> (`KismetArrayLibrary.Array_Length` (`self.MonstersAttackList`)) 0)
    (`KismetSystemLibrary.Delay` (+ (`KismetMathLibrary.RandomFloatInRange` 0.0 10.0) (`self.DelayBetweenAttacks`)))
    (set `self.CanAllowAttack` true)
    (`self.TryAllowNextMonsterAttack`)))

(fn `AddMonsterToAttackQueue`
  (params (MonsterBP :type "/Game/Blueprints/Act-1/Enemies/BP_Monster Object Reference (by ref)"))
  (bind _monsterspriority (`self.MonstersPriority`))
  (add `/Game/Blueprints/Act-1/Enemies/BP_Monster.OnAttackFinished` MonsterBP (`|CreateDelegate` :!event `RemoveMonsterFromQueue`))
  (bind (_arrayindex _arrayelement) (`/Engine/EditorBlueprintResources/StandardMacros.ReverseForEachLoop` (`self.MonstersAttackList`))
    (:`LoopBody`
      (if (> (`BlueprintMapLibrary.Map_Find` _monsterspriority (`/Game/Blueprints/Act-1/Enemies/BP_Monster.MonsterType` MonsterBP)) (`BlueprintMapLibrary.Map_Find` _monsterspriority (`/Game/Blueprints/Act-1/Enemies/BP_Monster.MonsterType` _arrayelement)))
        (if (== _arrayindex (`KismetArrayLibrary.Array_Length` (`self.MonstersAttackList`)))
          (`KismetArrayLibrary.Array_Add` (`self.MonstersAttackList`) MonsterBP)
          (else
            (`KismetArrayLibrary.Array_Insert` (`self.MonstersAttackList`) MonsterBP (+ _arrayindex 1))))
        (return)))
    (:`Completed`
      (`KismetSystemLibrary.PrintString` "eeeeeeeeeeeeeeeeeeeeeeeeeeeeeeeeeeeeeeeeeeeeeeeeeeeend"))))

(fn `RequestMonsterAttack`
  (params (Monster :type "/Game/Blueprints/Act-1/Enemies/BP_Monster Object Reference"))
  (if (and (== (`KismetArrayLibrary.Array_Length` (`self.MonstersAttackList`)) 0) (`self.CanAllowAttack`))
    (`self.AllowNextMonsterAttack` Monster)
    (else
      (`self.AddMonsterToAttackQueue` Monster))))

(fn `TryAllowNextMonsterAttack`
  (returns (Success :type Boolean))
  (if (`self.CanAllowAttack`)
    (`self.AllowNextMonsterAttack` (`|GetArrayItem` (`self.MonstersAttackList`)))
    (return true)
    (else
      (return false))))

(fn `UserConstructionScript`)