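; Base enemy logic for a monster that builds random progress toward a limit, then counts down to a jumpscare attack.
; Progress scales with rage and calmness modifiers, pauses during random delays or countdown, and nearing the limit starts the countdown that enables attacking.
; Tick only caches delta time, leaving the Try and Check steps to outside callers, while a one-second timer polls for countdown changes.
; Jumpscare and countdown-change hooks are empty.
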(event `self.ReceiveBeginPlay`
  (`KismetSystemLibrary.K2_SetTimer` null "CheckCountdown" 1.0 true))

(event `self.ReceiveTick`
  (params (DeltaSeconds :type "Float (single-precision)"))
  (set `self.DeltaTime` DeltaSeconds))

(event `InvokeResetMonster`
  (params (DelayTime :type "Float (double-precision)"))
  (`KismetSystemLibrary.Delay` DelayTime)
  (`self.ResetMonster`))

(event `OnCountdownChange`)

(fn `CheckCountdown`
  (if (not (== (`self.DoTimerCountdown`) (`self.PreciousCountdownValue`)))
    (`self.OnCountdownChange`))
  (set `self.PreciousCountdownValue` (`self.DoTimerCountdown`)))

(fn `CheckIfCanAttack`
  (bind _output_get (set `self.CanAttack` (<= (`self.TimeLeft`) 0.0)))
  (if _output_get
    (set `self.DoTimerCountdown` false)))

(fn `CheckProgress`
  (if (>= (`self.Progress`) (- (`self.ProgressLimit`) 3.0))
    (set `self.DoTimerCountdown` true)
    (if (`self.CanAttack`)
      (`self.TryDoJumpscare`))))

(fn `RandomProgressIncrease`
  (returns (Output_Get :type "Float (double-precision)"))
  (return (* (/ (* (* (`self.DeltaTime`) (`KismetMathLibrary.RandomFloatInRange` 0.0 1.0)) 100.0) (`self.CalmnessModifier`)) (* (`self.RandomRageModifier`) (`KismetMathLibrary.RandomFloatInRange` 0.0 6.0)))))

(fn `ResetMonster`
  (set `self.IsDelayed` false))

(fn `ResetRageModifier`
  (set `self.TimeLeft` 5.0)
  (set `self.RandomRageModifier` (`KismetMathLibrary.RandomFloatInRange` 1.0 3.0)))

(fn `SetNewLimit`
  (params (NewLimit :type "Float (double-precision)"))
  (set `self.ProgressLimit` NewLimit))

(fn `TryBlock`
  (if (<= (`KismetMathLibrary.RandomFloatInRange` 0.0 1.0) (`self.DelayChance`))
    (set `self.IsDelayed` true)
    (`self.InvokeResetMonster` (`KismetMathLibrary.RandomFloatInRange` 0.0 10.0))))

(fn `TryCountdown`
  (if (`self.DoTimerCountdown`)
    (set `self.TimeLeft` (- (`self.TimeLeft`) (`self.DeltaTime`)))
    (`self.CheckIfCanAttack`)))

(fn `TryDoJumpscare`)

(fn `TryIncrease`
  (if (and (== (`self.IsDelayed`) false) (== (`self.DoTimerCountdown`) false))
    (set `self.Progress` (`KismetMathLibrary.FClamp` (+ (`self.Progress`) (`self.RandomProgressIncrease`)) 0.0 (`self.ProgressLimit`)))))

(fn `UserConstructionScript`)