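; Door monster enemy for Act 1 that ends the game as a death when its jumpscare lands, built on a parent countdown and rage system.
; Countdown changes play a slow opening montage while the timer countdown is enabled.
; The jumpscare attempt succeeds only if the lamp is active, setting Death on the Act 1 game state.
; Otherwise it picks a random new limit and resets the rage modifier.
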(event `self.ReceiveBeginPlay`
  (`parent.ReceiveBeginPlay`)
  (`self.ResetRageModifier`))

(event `self.OnCountdownChange`
  (if (`self.DoTimerCountdown`)
    (`|PlayMontage` (`self.SkeletalMesh`) "/Game/Resources/Props/Environment/Room/Door/Animations/AM_OpeningSlow.AM_OpeningSlow")))

(fn `GetCanAttack`
  (returns (CanAttack :type Boolean))
  (return (`/Game/Blueprints/Act-1/Interactables/BP_Lamp.Active` (`self.Lamp`))))

(fn `TryDoJumpscare`
  (`parent.TryDoJumpscare`)
  (bind _canattack (`self.GetCanAttack`))
  (if _canattack
    (bind _asbp_base_night_game_state (cast `/Game/Blueprints/Act-1/Game/BP_Act-1GameState` (`GameplayStatics.GetGameState`)))
    (set `/Game/Blueprints/Act-1/Game/BP_Act-1GameState.Death` true _asbp_base_night_game_state)
    (`/Game/Blueprints/Act-1/Game/BP_Act-1GameState.EndGame` _asbp_base_night_game_state)
    (else
      (`self.SetNewLimit` (`KismetMathLibrary.RandomFloatInRange` 50.0 200.0))
      (`self.ResetRageModifier`))))

(fn `UserConstructionScript`
  (`parent.UserConstructionScript`))