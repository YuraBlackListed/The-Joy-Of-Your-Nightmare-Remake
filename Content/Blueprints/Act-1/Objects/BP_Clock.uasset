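; BP_Clock is an Act 1 clock object that displays the in-game hours and minutes.
; On BeginPlay it binds to the GameTimeSubsystem's hour and minute change events, which update separate HoursText and MinutesText elements without polling.
; Minutes get a leading zero only below ten, while hours always get one regardless of value.
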(event `self.ReceiveBeginPlay`
  (bind _returnvalue (subsystem `GameTimeSubsystem`))
  (add `GameTimeSubsystem.OnMinutesChanged` _returnvalue (delegate `OnMinutesChanged`))
  (add `GameTimeSubsystem.OnHoursChanged` _returnvalue (delegate `OnHoursChanged`)))

(event `OnMinutesChanged`
  (`TextRenderComponent.K2_SetText` (`self.MinutesText`) (`self.GetMinutes`)))

(event `OnHoursChanged`
  (`TextRenderComponent.K2_SetText` (`self.HoursText`) (`self.GetHours`)))

(fn `GetHours`
  (returns (HoursString :type Text))
  (return (`KismetTextLibrary.Conv_StringToText` (`KismetStringLibrary.Concat_StrStr` "0" (`KismetStringLibrary.Conv_IntToString` (`GameTimeSubsystem.GetHours` (subsystem `GameTimeSubsystem`)))))))

(fn `GetMinutes`
  (returns (MinutesString :type Text))
  (bind _returnvalue (`GameTimeSubsystem.GetMinutes` (subsystem `GameTimeSubsystem`)))
  (bind _returnvalue_2 (`KismetStringLibrary.Conv_IntToString` _returnvalue))
  (if (< _returnvalue 10)
    (return (`KismetTextLibrary.Conv_StringToText` (`KismetStringLibrary.Concat_StrStr` "0" _returnvalue_2)))
    (else
      (return (`KismetTextLibrary.Conv_StringToText` _returnvalue_2)))))

(fn `UserConstructionScript`)