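; BP_GameInfoInstance is a game-info hub, apparently the Game Instance, that shows shared UI screens: main menu, tutorial hint and fade transition.
; Each Show event lazily creates and caches its widget, adds it to the viewport and shows the mouse cursor.
; FadeIn and FadeOut create the transition screen if missing; the hint screen also pauses the game and clears other widgets.
; Save checking, options, loading and error handling are stubs.
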(event `CheckForSaveGame`
  (bind _returnvalue (`GameplayStatics.DoesSaveGameExist` (`self.PlayerSettingsSave`)))
  (if _returnvalue
    _))

(event `FadeIn`
  (bind _wb_fadescreen (`self.WB_FadeScreen`))
  (`/Engine/EditorBlueprintResources/StandardMacros.IsValid` _wb_fadescreen
    (:`Is Valid`
      _)
    (:`Is Not Valid`
      (`self.ShowFadeScreen`)))
  (`/Game/UI/LoadingScreen/WB_TransitionScreen.OnFadeIn` _wb_fadescreen))

(event `FadeOut`
  (bind _wb_fadescreen (`self.WB_FadeScreen`))
  (`/Engine/EditorBlueprintResources/StandardMacros.IsValid` _wb_fadescreen
    (:`Is Valid`
      _)
    (:`Is Not Valid`
      (`self.ShowFadeScreen`)))
  (`/Game/UI/LoadingScreen/WB_TransitionScreen.OnFadeOut` _wb_fadescreen))

(event `ShowFadeScreen`
  (bind _returnvalue (`GameplayStatics.GetPlayerController` 0))
  (bind _wb_fadescreen (`self.WB_FadeScreen`))
  (`/Engine/EditorBlueprintResources/StandardMacros.IsValid` _wb_fadescreen
    (:`Is Valid`
      _)
    (:`Is Not Valid`
      (bind _returnvalue_2 (`|CreateWidget` "/Game/UI/LoadingScreen/WB_TransitionScreen.WB_TransitionScreen_C" _returnvalue))
      (bind _output_get (set `self.WB_FadeScreen` _returnvalue_2))))
  (`UserWidget.AddToViewport` _wb_fadescreen 0)
  (`UserWidget.AddToViewport` _output_get 0)
  (set `PlayerController.bShowMouseCursor` true _returnvalue))

(event `ShowHintScreen`
  (bind _returnvalue (`GameplayStatics.GetPlayerController` 0))
  (bind _wb_hintscreen (`self.WB_HintScreen`))
  (`GameplayStatics.SetGamePaused` true)
  (`WidgetLayoutLibrary.RemoveAllWidgets`)
  (`/Engine/EditorBlueprintResources/StandardMacros.IsValid` _wb_hintscreen
    (:`Is Valid`
      _)
    (:`Is Not Valid`
      (bind _returnvalue_2 (`|CreateWidget` "/Game/UI/LoadingScreen/WB_TutorialScreen.WB_TutorialScreen_C" _returnvalue))
      (bind _output_get (set `self.WB_HintScreen` _returnvalue_2))))
  (`UserWidget.AddToViewport` _wb_hintscreen 0)
  (`UserWidget.AddToViewport` _output_get 0)
  (set `PlayerController.bShowMouseCursor` true _returnvalue))

(event `ShowMainMenu`
  (bind _returnvalue (`GameplayStatics.GetPlayerController` 0))
  (bind _wb_mainmenu (`self.WB_MainMenu`))
  (`/Engine/EditorBlueprintResources/StandardMacros.IsValid` _wb_mainmenu
    (:`Is Valid`
      _)
    (:`Is Not Valid`
      (bind _returnvalue_2 (`|CreateWidget` "/Game/UI/MainMenu/WB_MainMenu.WB_MainMenu_C" _returnvalue))
      (set `self.WB_MainMenu` _returnvalue_2)))
  (`UserWidget.AddToViewport` _wb_mainmenu 0)
  (set `PlayerController.bShowMouseCursor` true _returnvalue))

(event `ShowOptionsMenu`)

(event `ShowLoadingScreen`)

(fn `NetErrorToString`
  (params (FailureType :type "ENetworkFailure Enum" :default "NetDriverAlreadyExists"))
  (returns (OutString :type String))
  (return ""))

(fn `TravelErrorToString`
  (params (FailureType :type "ETravelFailure Enum" :default "NoLevel"))
  (returns (OutString :type String))
  (return ""))