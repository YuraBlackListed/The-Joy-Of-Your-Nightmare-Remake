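; Player component that detects interactable actors under the camera's view and forwards interaction input to them.
; Each tick a Visibility line trace runs from the camera out to InteractDistance, caching any hit actor that implements BPI_Interactable.
; Start or stop hover is called every tick based on that result, not just on changes.
; Press, hold and release inputs call StartInteraction, Interact and StopInteraction on the cached target while it is valid.
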(event `self.ReceiveTick`
  (params (DeltaSeconds :type "Float (single-precision)"))
  (`self.TryFindInteractable`)
  (if (`self.InteractableIsValid`)
    (`self.OnInteractableStartHover`)
    (else
      (`self.OnInteractableStopHover`))))

(event `EnhancedInput|/Game/Data/Input/Act-1/InputActions/IA_StartInteraction`
  (params (ActionValue :type Boolean) (ElapsedSeconds :type "Float (double-precision)") (TriggeredSeconds :type "Float (double-precision)") (InputAction :type "InputAction Object Reference" :default "/Game/Data/Input/Act-1/InputActions/IA_StartInteraction.IA_StartInteraction"))
  (:`Triggered`
    (`self.TryInteract` "NewEnumerator0")))

(event `EnhancedInput|/Game/Data/Input/Act-1/InputActions/IA_HoldInteraction`
  (params (ActionValue :type Boolean) (ElapsedSeconds :type "Float (double-precision)") (TriggeredSeconds :type "Float (double-precision)") (InputAction :type "InputAction Object Reference" :default "/Game/Data/Input/Act-1/InputActions/IA_HoldInteraction.IA_HoldInteraction"))
  (:`Triggered`
    (`self.TryInteract` "NewEnumerator1")))

(event `EnhancedInput|/Game/Data/Input/Act-1/InputActions/IA_StopInteraction`
  (params (ActionValue :type Boolean) (ElapsedSeconds :type "Float (double-precision)") (TriggeredSeconds :type "Float (double-precision)") (InputAction :type "InputAction Object Reference" :default "/Game/Data/Input/Act-1/InputActions/IA_StopInteraction.IA_StopInteraction"))
  (:`Triggered`
    (`self.TryInteract` "NewEnumerator2")))

(fn `GetTraceVectors`
  (returns (Start :type "Vector Structure") (End :type "Vector Structure"))
  (bind _playercameramanager (`PlayerController.PlayerCameraManager` (`GameplayStatics.GetPlayerController` 0)))
  (bind _returnvalue (`PlayerCameraManager.GetCameraLocation` _playercameramanager))
  (return _returnvalue (+ _returnvalue (* (`KismetMathLibrary.GetForwardVector` (`PlayerCameraManager.GetCameraRotation` _playercameramanager)) (`self.InteractDistance`)))))

(fn `TryFindInteractable`
  (bind (_start _end) (`self.GetTraceVectors`))
  (bind (_outhit _returnvalue) (`KismetSystemLibrary.LineTraceSingle` :`Start` _start :`End` _end :`TraceChannel` "TraceTypeQuery1" :`DrawTime` 2.0))
  (if _returnvalue
    (bind _asbpi_interactable (cast `/Game/Blueprints/General/Interactables/BPI_Interactable` (`.HitActor` (`GameplayStatics.BreakHitResult` _outhit)))
      (:`then`
        (set `self.LastInteractable` _asbpi_interactable)
        (set `self.InteractableIsValid` true))
      (:`CastFailed`
        (set `self.InteractableIsValid` false :!label _label)))
    (else
      (goto _label))))

(fn `TryInteract`
  (params (InteractionType :type "/Game/Blueprints/General/Interactables/E_InteractionType Enum" :default "NewEnumerator0"))
  (bind _lastinteractable (`self.LastInteractable`))
  (if (`self.InteractableIsValid`)
    (switch `/Game/Blueprints/General/Interactables/E_InteractionType` InteractionType
      (:`NewEnumerator0`
        (`/Game/Blueprints/General/Interactables/BPI_Interactable.StartInteraction` _lastinteractable))
      (:`NewEnumerator1`
        (`/Game/Blueprints/General/Interactables/BPI_Interactable.Interact` _lastinteractable))
      (:`NewEnumerator2`
        (`/Game/Blueprints/General/Interactables/BPI_Interactable.StopInteraction` _lastinteractable)))))