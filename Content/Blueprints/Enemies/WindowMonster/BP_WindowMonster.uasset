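; BP_WindowMonster is a child enemy that kills the player through an open window during a night.
; A countdown change event activates it, and its TryDoJumpscare override runs the parent logic, then checks whether its Window is open.
; An open window flags death on the night game state and ends the game.
; A closed one sets a new random limit and resets the rage modifier; both outcomes deactivate the monster.
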(event `self.ReceiveBeginPlay`
  (`parent.ReceiveBeginPlay`)
  (`self.ResetRageModifier`))

(event `self.OnCountdownChange`
  (set `self.Activated` true))

(fn `GetCanAttack`
  (returns (CanAttack :type Boolean))
  (return (`/Game/Blueprints/Interactables/BP_Curtains.Opened` (`self.Window`))))

(fn `TryDoJumpscare`
  (`parent.TryDoJumpscare`)
  (`self.TryDoWindowJumpscare`))

(fn `TryDoWindowJumpscare`
  (bind _canattack (`self.GetCanAttack`))
  (if _canattack
    (bind _asbp_base_night_game_state (cast `/Game/Blueprints/Game/BP_BaseNightGameState` (`GameplayStatics.GetGameState`)))
    (set `/Game/Blueprints/Game/BP_BaseNightGameState.Death` true _asbp_base_night_game_state)
    (`/Game/Blueprints/Game/BP_BaseNightGameState.EndGame` _asbp_base_night_game_state)
    (else
      (`self.SetNewLimit` (`KismetMathLibrary.RandomFloatInRange` 50.0 200.0))
      (`self.ResetRageModifier`)))
  (set `self.Activated` false))

(fn `UserConstructionScript`
  (`parent.UserConstructionScript`))