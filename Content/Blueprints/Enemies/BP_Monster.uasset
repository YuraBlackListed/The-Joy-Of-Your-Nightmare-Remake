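; Base enemy monster for the night game mode, which caches the night game state and starts its behavior tree on BeginPlay.
; It can subscribe to the game state's next-attack dispatcher, attempts a jumpscare when it is the allowed monster, and binds unsubscription to its attack finishing.
; Rage helpers expose the progress limit, multiplier, attack flag and a random modifier reset.
; The jumpscare and countdown hooks are empty here.
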(event `self.ReceiveBeginPlay`
  (bind _asbp_base_night_game_state (cast `/Game/Blueprints/Game/BP_BaseNightGameState` (`GameplayStatics.GetGameState`)))
  (set `self.As BP Base Night Game State` _asbp_base_night_game_state)
  (`BrainComponent.StartLogic` (`self.BehaviorTree`)))

(event `self.ReceiveTick`
  (params (DeltaSeconds :type "Float (single-precision)"))
  (set `self.DeltaTime` DeltaSeconds))

(event `OnCountdownChange`)

(event `AssignOnLetNextMonsterAttackEvent`
  (add `/Game/Blueprints/Game/BP_BaseNightGameState.AllowNextMonsterAttack` (`self.As BP Base Night Game State`) (delegate `CheckAllowedMonsterToAttack`)))

(event `CheckAllowedMonsterToAttack`
  (params (Monster :type "/Game/Blueprints/Enemies/BP_Monster Object Reference"))
  (if (== Monster self)
    (add `self.OnAttackFinished` (delegate `UnsubscribeFromAllowedMonsterToAttackevent`))
    (`self.TryDoJumpscare`)))

(event `UnsubscribeFromAllowedMonsterToAttackevent`
  (remove `/Game/Blueprints/Game/BP_BaseNightGameState.AllowNextMonsterAttack` (`self.As BP Base Night Game State`) (delegate `CheckAllowedMonsterToAttack`)))

(fn `GetCanAttack`
  (returns (CanAttack :type Boolean))
  (return (`self.CanAttack`)))

(fn `GetRageLimit`
  (returns (RageLimit :type "Float (double-precision)"))
  (return (`self.ProgressLimit`)))

(fn `GetRageMultiplier`
  (returns (Multiplier :type "Float (double-precision)"))
  (return (`self.ProgressMultiplier`)))

(fn `ResetRageModifier`
  (set `self.RandomRageModifier` (`KismetMathLibrary.RandomFloatInRange` 1.0 3.0)))

(fn `SetNewLimit`
  (params (NewLimit :type "Float (double-precision)"))
  (set `self.ProgressLimit` NewLimit))

(fn `TryDoJumpscare`)

(fn `UserConstructionScript`)