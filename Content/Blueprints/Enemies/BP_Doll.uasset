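; BP_Doll is an enemy that layers window-dependent behavior onto its parent's jumpscare and countdown logic.
; A looping 0.75-second timer calls TryIncrease, while Tick checks progress and runs the countdown.
; Its jumpscare override calls the parent, then, if the window is open, resets progress and rage, stops the countdown and picks a random new limit.
; ActivateAnimation sets an Activated flag, which the window check always clears.
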(event `self.ReceiveBeginPlay`
  (`parent.ReceiveBeginPlay`)
  (`self.TryBlock`)
  (`self.ResetRageModifier`)
  (`KismetSystemLibrary.K2_SetTimer` null "TryIncrease" 0.75 true))

(event `self.ReceiveTick`
  (params (DeltaSeconds :type "Float (single-precision)"))
  (`parent.ReceiveTick` DeltaSeconds)
  (`self.CheckProgress`)
  (`self.TryCountdown`))

(event `self.ActivateAnimation`
  (set `self.Activated` true))

(fn `TryCountdown`
  (`parent.TryCountdown`))

(fn `TryDoJumpscare`
  (`parent.TryDoJumpscare`)
  (`self.TryDoWindowJumpscare`))

(fn `TryDoWindowJumpscare`
  (if (`/Game/Blueprints/Interactables/BP_Curtains.Opened` (`self.Window`))
    (set `self.Progress` 0.0)
    (set `self.DoTimerCountdown` false)
    (`self.SetNewLimit` (`KismetMathLibrary.RandomFloatInRange` 50.0 200.0))
    (`self.ResetRageModifier`))
  (set `self.Activated` false))

(fn `UserConstructionScript`
  (`parent.UserConstructionScript`))