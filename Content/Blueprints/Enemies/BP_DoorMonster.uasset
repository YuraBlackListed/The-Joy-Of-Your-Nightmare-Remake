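; BP_DoorMonster is a child enemy Blueprint for a door monster with a progress, countdown and jumpscare cycle, mostly handled by its parent.
; BeginPlay starts a looping TryIncrease timer, while Tick runs the inherited progress and countdown checks.
; An active countdown triggers the slow-opening montage.
; After the parent's jumpscare attempt, an inactive Lamp resets progress, countdown, attack and rage state and picks a new random limit.
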(event `self.ReceiveBeginPlay`
  (`parent.ReceiveBeginPlay`)
  (`self.TryBlock`)
  (`self.ResetRageModifier`)
  (`KismetSystemLibrary.K2_SetTimer` null "TryIncrease" 1.0 true))

(event `self.ReceiveTick`
  (params (DeltaSeconds :type "Float (single-precision)"))
  (`parent.ReceiveTick` DeltaSeconds)
  (`self.CheckProgress`)
  (`self.TryCountdown`))

(event `self.OnCountdownChange`
  (if (`self.DoTimerCountdown`)
    (`|PlayMontage` (`self.SkeletalMesh`) "/Game/Meshes/Environment/Room/Door/Animations/AM_OpeningSlow.AM_OpeningSlow")))

(fn `CheckProgress`
  (`parent.CheckProgress`))

(fn `TryCountdown`
  (`parent.TryCountdown`))

(fn `TryDoJumpscare`
  (`parent.TryDoJumpscare`)
  (if (not (`/Game/Blueprints/Interactables/BP_Lamp.Active` (`self.Lamp`)))
    (set `self.Progress` 0.0)
    (set `self.DoTimerCountdown` false)
    (set `self.CanAttack` false)
    (`self.SetNewLimit` (`KismetMathLibrary.RandomFloatInRange` 50.0 200.0))
    (`self.ResetRageModifier`)))

(fn `UserConstructionScript`
  (`parent.UserConstructionScript`))