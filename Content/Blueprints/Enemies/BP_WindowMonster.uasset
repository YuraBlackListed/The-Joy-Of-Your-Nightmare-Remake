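; BP_WindowMonster is an enemy that threatens the player through a window, ending the game if its attack finds that window open.
; A looping timer calls TryIncrease, while Tick runs progress and countdown checks, and a countdown change marks it activated.
; Its jumpscare extends the parent's: an open window triggers death through the Act-1 game state, while a closed one resets progress, countdown and rage, and rolls a new random limit.
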(event `self.ReceiveBeginPlay`
  (`parent.ReceiveBeginPlay`)
  (`self.TryBlock`)
  (`self.ResetRageModifier`)
  (`KismetSystemLibrary.K2_SetTimer` null "TryIncrease" 0.75 true))

(event `self.ReceiveTick`
  (params (DeltaSeconds :type "Float (single-precision)"))
  (`parent.ReceiveTick` DeltaSeconds)
  (`self.CheckProgress`)
  (`self.TryCountdown`))

(event `self.OnCountdownChange`
  (set `self.Activated` true))

(fn `TryCountdown`
  (`parent.TryCountdown`))

(fn `TryDoJumpscare`
  (`parent.TryDoJumpscare`)
  (`self.TryDoWindowJumpscare`))

(fn `TryDoWindowJumpscare`
  (if (`/Game/Blueprints/Interactables/BP_Curtains.Opened` (`self.Window`))
    (bind _asbp_act_1game_state (cast `/Game/Blueprints/Game/BP_Act-1GameState` (`GameplayStatics.GetGameState`)))
    (set `/Game/Blueprints/Game/BP_Act-1GameState.Death` true _asbp_act_1game_state)
    (`/Game/Blueprints/Game/BP_Act-1GameState.EndGame` _asbp_act_1game_state)
    (else
      (set `self.Progress` 0.0)
      (set `self.DoTimerCountdown` false)
      (set `self.CanAttack` false)
      (`self.SetNewLimit` (`KismetMathLibrary.RandomFloatInRange` 50.0 200.0))
      (`self.ResetRageModifier`)))
  (set `self.Activated` false))

(fn `UserConstructionScript`
  (`parent.UserConstructionScript`))