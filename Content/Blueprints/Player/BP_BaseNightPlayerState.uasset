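; Night-mode player state that drives fear feedback through post-process, camera shake and heartbeat audio.
; It toggles its lights flag on the game state's darkness-change event.
; While lights are off, Tick compounds FearLevel by a multiplier and feeds it through curves into chromatic aberration, film grain, focal distance and shake scale.
; A looked-up curve also sets the heartbeat's fear submix send every tick, regardless of lighting.
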(event `self.ReceiveBeginPlay`
  (bind _asbp_base_night_game_state (cast `/Game/Blueprints/Game/BP_BaseNightGameState` (`GameplayStatics.GetGameState`)))
  (bind _output_get (set `self.GameState` _asbp_base_night_game_state))
  (add `/Game/Blueprints/Game/BP_BaseNightGameState.DarknessChange` _output_get (delegate `SwitchDarkness`))
  (bind _returnvalue (`PlayerCameraManager.StartCameraShake` :`self` (`GameplayStatics.GetPlayerCameraManager` 0) :`ShakeClass` "/Game/Blueprints/Camera/BP_CameraShake.BP_CameraShake_C"))
  (set `self.CameraShake` _returnvalue)
  (set `CameraShakeBase.ShakeScale` 0.0 (`self.CameraShake`))
  (bind _returnvalue_2 (`GameplayStatics.SpawnSound2D` "/Game/Sounds/Effects/SC_Heartbeating.SC_Heartbeating" 1.0 1.0 0.0 null))
  (bind _output_get_2 (set `self.AudioComponent` _returnvalue_2))
  (`AudioComponent.SetSubmixSend` _output_get_2 "/Game/Sounds/SS_Fear.SS_Fear" 0.0))

(event `SwitchDarkness`
  (set `self.LightsOn` (not (`self.LightsOn`))))

(event `self.ReceiveTick`
  (params (DeltaSeconds :type "Float (single-precision)"))
  (`self.UpdateAllVisualEffects`)
  (`self.UpdateHeartbeatVolume`))

(fn `UpdateAllVisualEffects`
  (if (not (`self.LightsOn`))
    (set `self.FearLevel` (* (`self.FearLevel`) (`self.FearModifier`)))
    (setmembers `PostProcessSettings` :`StructRef` (`PostProcessVolume.Settings` (`self.PostProcess`)) :`SceneFringeIntensity` (`CurveFloat.GetFloatValue` (`self.ChromaticAberration`) (`self.FearLevel`)) :`FilmGrainTexelSize` (`CurveFloat.GetFloatValue` (`self.FilmGrainCurve`) (`self.FearLevel`)) :`DepthOfFieldFocalDistance` (`CurveFloat.GetFloatValue` (`self.FocalDistance`) (`self.FearLevel`)))
    (set `CameraShakeBase.ShakeScale` (`CurveFloat.GetFloatValue` (`self.CameraShakeCurve`) (`self.FearLevel`)) (`self.CameraShake`))))

(fn `UpdateHeartbeatVolume`
  (`AudioComponent.SetSubmixSend` (`self.AudioComponent`) "/Game/Sounds/SS_Fear.SS_Fear" (`CurveFloat.GetFloatValue` (`self.SoundVolume`) (`self.FearLevel`))))

(fn `UserConstructionScript`)