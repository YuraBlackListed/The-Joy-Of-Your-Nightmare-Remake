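; BP_Player is the player Blueprint, with mouse-look, leaning, interaction and a jumpscare.
; The camera rides a socket on Body, with pitch clamped to straight up and down.
; The lean input toggles window or drawer lean flags based on camera yaw, while interact inputs forward to ACInteractionTrace.
; OnJumpscare places and activates ScreamerBody at the camera, locks look input and sets the FOV.
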(event `self.ReceiveBeginPlay`
  (`SceneComponent.K2_AttachToComponent` (`self.Camera`) (`self.Body`) "CameraSocket" "KeepRelative" "KeepRelative" "KeepRelative" true)
  (`ActorComponent.SetActive` (`self.ScreamerBody`) false false))

(event `EnhancedInput|/Game/Input/Actions/IA_Look`
  (params (ActionValue :type "Vector2D Structure") (ElapsedSeconds :type "Float (double-precision)") (TriggeredSeconds :type "Float (double-precision)") (InputAction :type "InputAction Object Reference" :default "/Game/Input/Actions/IA_Look.IA_Look"))
  (bind _camera (`self.Camera`))
  (bind (_relativerotation_roll _relativerotation_pitch _relativerotation_yaw) (`KismetMathLibrary.BreakRotator` (`SceneComponent.RelativeRotation` _camera)))
  (bind _returnvalue (- _relativerotation_pitch ActionValue_Y))
  (:`Triggered`
    (if (`self.Screamer`)
      _
      (elif (<= _returnvalue 90.0)
        (if (>= _returnvalue -90.0)
          (`SceneComponent.K2_SetRelativeRotation` _camera (`KismetMathLibrary.MakeRotator` 0.0 _returnvalue (+ _relativerotation_yaw ActionValue_X)) true false))))))

(event `EnhancedInput|/Game/Input/Actions/IA_LeanToSide`
  (params (ActionValue :type Boolean) (ElapsedSeconds :type "Float (double-precision)") (TriggeredSeconds :type "Float (double-precision)") (InputAction :type "InputAction Object Reference" :default "/Game/Input/Actions/IA_LeanToSide.IA_LeanToSide"))
  (:`Triggered`
    (`self.ChooseSideToLeanTo`)))

(event `EnhancedInput|/Game/Input/Actions/IA_Interact`
  (params (ActionValue :type Boolean) (ElapsedSeconds :type "Float (double-precision)") (TriggeredSeconds :type "Float (double-precision)") (InputAction :type "InputAction Object Reference" :default "/Game/Input/Actions/IA_Interact.IA_Interact"))
  (:`Triggered`
    (`/Game/Blueprints/Player/AC_InteractionTrace.TryInteract` (`self.AC_InteractionTrace`))))

(event `EnhancedInput|/Game/Input/Actions/IA_UnInteract`
  (params (ActionValue :type Boolean) (ElapsedSeconds :type "Float (double-precision)") (TriggeredSeconds :type "Float (double-precision)") (InputAction :type "InputAction Object Reference" :default "/Game/Input/Actions/IA_UnInteract.IA_UnInteract"))
  (:`Triggered`
    (`/Game/Blueprints/Player/AC_InteractionTrace.TryUninteract` (`self.AC_InteractionTrace`))))

(event `OnJumpscare`
  (bind _returnvalue (`SceneComponent.K2_GetComponentToWorld` (`self.Camera`)))
  (`SceneComponent.K2_SetWorldTransform` (`self.ScreamerBody`) (`KismetMathLibrary.MakeTransform` (.location _returnvalue) (`KismetMathLibrary.MakeRotator` (.roll (.rotation _returnvalue)) (.pitch (.rotation _returnvalue)) (+ (.yaw (.rotation _returnvalue)) 90.0))) false false)
  (`ActorComponent.SetActive` (`self.ScreamerBody`) true false)
  (set `self.Screamer` true)
  (`CameraComponent.SetFieldOfView` (`self.Camera`) 60.0))

(fn `CheckIfCameraRotationInRange`
  (params (Min :type "Float (double-precision)") (Max :type "Float (double-precision)"))
  (returns (ReturnValue :type Boolean))
  (bind (_relativerotation_roll _relativerotation_pitch _relativerotation_yaw) (`KismetMathLibrary.BreakRotator` (`SceneComponent.RelativeRotation` (`self.Camera`))))
  (return (`KismetMathLibrary.InRange_FloatFloat` _relativerotation_yaw Min Max)))

(fn `ChooseSideToLeanTo`
  (if (or (`self.LeaningWindow`) (`self.LeaningDrawer`))
    (`self.CheckIfCameraRotationInRange` -180.0 180.0)
    (set `self.LeaningWindow` false)
    (set `self.LeaningDrawer` false)
    (else
      (`|ExecutionSequence`
        (:`then_0`
          (bind _returnvalue (`self.CheckIfCameraRotationInRange` -30.0 40.0))
          (set `self.LeaningWindow` _returnvalue))
        (:`then_1`
          (bind _returnvalue_2 (`self.CheckIfCameraRotationInRange` 40.0 80.0))
          (set `self.LeaningDrawer` _returnvalue_2))))))

(fn `UserConstructionScript`)