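; Player component that detects the interactable under the crosshair and forwards interact and uninteract requests to it.
; Each tick it line-traces on Visibility from the camera out to a reach distance, re-evaluating when the hit actor changes.
; Only actors of exactly the BP_Interactable class qualify, updating the crosshair.
; Losing the target triggers uninteract on the cached interactable, then clears it.
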(event `self.ReceiveTick`
  (params (DeltaSeconds :type "Float (single-precision)"))
  (`self.Trace`))

(event `TryInteract`
  (if (`self.IsInteractableTraced`)
    (message `/Game/Blueprints/Interactables/BPI_Interactable.Interact` (`self.Interactable`))))

(event `TryUninteract`
  (bind _interactable (`self.Interactable`))
  (if (not (`self.IsInteractableTraced`))
    (`/Engine/EditorBlueprintResources/StandardMacros.IsValid` _interactable
      (:`Is Valid`
        _)))
  (`/Game/Blueprints/Interactables/BPI_Interactable.UnInteract` _interactable))

(fn `Trace`
  (bind _returnvalue (`GameplayStatics.GetPlayerCameraManager` 0))
  (bind _returnvalue_2 (`Actor.K2_GetActorLocation` _returnvalue))
  (bind (_outhit _returnvalue_3) (`KismetSystemLibrary.LineTraceSingle` :`Start` _returnvalue_2 :`End` (+ _returnvalue_2 (* (`KismetMathLibrary.GetForwardVector` (`Actor.K2_GetActorRotation` _returnvalue)) (`self.ReachDistance`))) :`TraceChannel` "TraceTypeQuery1" :`TraceColor` (struct :`G` 0.359283 :`B` 1.0 :`A` 1.0)))
  (if _returnvalue_3
    (bind (_bblockinghit _binitialoverlap _time _distance _location _impactpoint _normal _impactnormal _physmat _hitactor) (`GameplayStatics.BreakHitResult` _outhit))
    (if (!= (`self.FocusedActor`) _hitactor)
      (set `self.FocusedActor` _hitactor)
      (`self.TraceInteractibleArea` (== (`GameplayStatics.GetObjectClass` _hitactor) "/Game/Blueprints/Interactables/BP_Interactable.BP_Interactable_C")))
    (else
      (`self.TraceInteractibleArea` false))))

(fn `TraceInteractibleArea`
  (params (Trace :type Boolean))
  (if Trace
    (if (`self.IsInteractableTraced`)
      (`self.CrosshairChange` (`self.IsInteractableTraced`)))
    (bind _asbp_interactable (cast `/Game/Blueprints/Interactables/BP_Interactable` (`self.FocusedActor`)))
    (set `self.Interactable` _asbp_interactable)
    (bind _output_get (set `self.IsInteractableTraced` true))
    (`self.CrosshairChange` _output_get)
    (elif (`self.IsInteractableTraced`)
      (set `self.IsInteractableTraced` false)
      (`self.CrosshairChange` (`self.IsInteractableTraced`))
      (`self.TryUnInteract`)
      (set `self.Interactable` null)
      (set `self.FocusedActor` null))))