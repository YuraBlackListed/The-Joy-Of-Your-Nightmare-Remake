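; Game instance (by name) that owns screen widgets, level transitions and saving of night progress.
; Show events lazily create and cache fade, white, hint and main menu widgets; the hint screen also pauses the game.
; LoadLevel fades in, shows a loading screen after a delay, then opens the level.
; WinSaveGame increments Night on a fresh save object, saves it and opens MainMenu; save checking, options and error handlers are stubs.
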(event `CheckForSaveGame`
  (bind _returnvalue (`GameplayStatics.DoesSaveGameExist` (`self.PlayerSettingsSave`)))
  (if _returnvalue
    _))

(event `FadeIn`
  (`self.ShowTransitionScreen`)
  (`/Game/Blueprints/Menu/UI/LoadingScreen/WBP_TransitionScreen.OnFadeIn` (`self.WB_FadeScreen`)))

(event `FadeOut`
  (`self.ShowTransitionScreen`)
  (`/Game/Blueprints/Menu/UI/LoadingScreen/WBP_TransitionScreen.OnFadeOut` (`self.WB_FadeScreen`)))

(event `LoadLevel`
  (params (Level :type "World Soft Object Reference"))
  (`self.FadeIn`)
  (`KismetSystemLibrary.Delay` 2.0)
  (bind _returnvalue (`|CreateWidget` "/Game/Blueprints/Menu/UI/LoadingScreen/WBP_LoadingScreen.WBP_LoadingScreen_C" (`GameplayStatics.GetPlayerController` 0)))
  (`UserWidget.AddToViewport` _returnvalue 0)
  (`KismetSystemLibrary.Delay` 1.0)
  (`GameplayStatics.OpenLevelBySoftObjectPtr` Level))

(event `ShowTransitionScreen`
  (bind _returnvalue (`GameplayStatics.GetPlayerController` 0))
  (bind _wb_fadescreen (`self.WB_FadeScreen`))
  (`/Engine/EditorBlueprintResources/StandardMacros.IsValid` _wb_fadescreen
    (:`Is Valid`
      _)
    (:`Is Not Valid`
      (bind _returnvalue_2 (`|CreateWidget` "/Game/Blueprints/Menu/UI/LoadingScreen/WBP_TransitionScreen.WBP_TransitionScreen_C" _returnvalue))
      (bind _output_get (set `self.WB_FadeScreen` _returnvalue_2))))
  (`UserWidget.AddToViewport` _wb_fadescreen 0)
  (`UserWidget.AddToViewport` _output_get 0)
  (set `PlayerController.bShowMouseCursor` true _returnvalue))

(event `ShowWhiteScreen`
  (bind _wb_whitescreen (`self.WB_WhiteScreen`))
  (`/Engine/EditorBlueprintResources/StandardMacros.IsValid` _wb_whitescreen
    (:`Is Valid`
      _)
    (:`Is Not Valid`
      (bind _returnvalue (`|CreateWidget` "/Game/Blueprints/Menu/UI/LoadingScreen/WBP_WhiteTransition.WBP_WhiteTransition_C" (`GameplayStatics.GetPlayerController` 0)))
      (bind _output_get (set `self.WB_WhiteScreen` _returnvalue))))
  (`UserWidget.AddToViewport` _wb_whitescreen 0)
  (`UserWidget.AddToViewport` _output_get 0))

(event `ShowHintScreen`
  (bind _returnvalue (`GameplayStatics.GetPlayerController` 0))
  (bind _wb_hintscreen (`self.WB_HintScreen`))
  (`GameplayStatics.SetGamePaused` true)
  (`WidgetLayoutLibrary.RemoveAllWidgets`)
  (`/Engine/EditorBlueprintResources/StandardMacros.IsValid` _wb_hintscreen
    (:`Is Valid`
      _)
    (:`Is Not Valid`
      (bind _returnvalue_2 (`|CreateWidget` "/Game/Blueprints/Menu/UI/LoadingScreen/WBP_TutorialScreen.WBP_TutorialScreen_C" _returnvalue))
      (bind _output_get (set `self.WB_HintScreen` _returnvalue_2))))
  (`UserWidget.AddToViewport` _wb_hintscreen 0)
  (`UserWidget.AddToViewport` _output_get 0)
  (set `PlayerController.bShowMouseCursor` true _returnvalue))

(event `ShowMainMenu`
  (bind _returnvalue (`GameplayStatics.GetPlayerController` 0))
  (bind _wb_mainmenu (`self.WB_MainMenu`))
  (`/Engine/EditorBlueprintResources/StandardMacros.IsValid` _wb_mainmenu
    (:`Is Valid`
      _)
    (:`Is Not Valid`
      (bind _returnvalue_2 (`|CreateWidget` "/Game/Blueprints/Menu/UI/WBP_MainMenu.WBP_MainMenu_C" _returnvalue))
      (set `self.WB_MainMenu` _returnvalue_2)))
  (`UserWidget.AddToViewport` _wb_mainmenu 0)
  (set `PlayerController.bShowMouseCursor` true _returnvalue))

(event `ShowLoadingScreen`
  (bind _returnvalue (`|CreateWidget` "/Game/Blueprints/Menu/UI/LoadingScreen/WBP_LoadingScreen.WBP_LoadingScreen_C" (`GameplayStatics.GetPlayerController` 0)))
  (`UserWidget.AddToViewport` _returnvalue 0))

(event `ShowOptionsMenu`)

(fn `NetErrorToString`
  (params (FailureType :type "ENetworkFailure Enum" :default "NetDriverAlreadyExists"))
  (returns (OutString :type String))
  (return ""))

(fn `SaveGame`
  (params (Night :type Integer) (PlayerSaveGame :type "/Game/Blueprints/SaveSystem/BP_PlayerSaveGame Object Reference"))
  (set `/Game/Blueprints/SaveSystem/BP_PlayerSaveGame.PlayerInfo` (make `/Game/Blueprints/SaveSystem/S_PlayerInfo` Night) PlayerSaveGame)
  (`GameplayStatics.SaveGameToSlot` PlayerSaveGame (`self.PlayerSettingsSave`)))

(fn `TravelErrorToString`
  (params (FailureType :type "ETravelFailure Enum" :default "NoLevel"))
  (returns (OutString :type String))
  (return ""))

(fn `WinSaveGame`
  (bind _returnvalue (`GameplayStatics.CreateSaveGameObject` "/Game/Blueprints/SaveSystem/BP_PlayerSaveGame.BP_PlayerSaveGame_C"))
  (bind _result (`/Engine/EditorBlueprintResources/StandardMacros.IncrementInt` (`.Night_5_A32BE8E743FBA272A8E3C187CE0984FB` (break `/Game/Blueprints/SaveSystem/S_PlayerInfo` (`/Game/Blueprints/SaveSystem/BP_PlayerSaveGame.PlayerInfo` _returnvalue))))
    (:`  `
      (`self.SaveGame` _result _returnvalue)
      (`GameplayStatics.OpenLevelBySoftObjectPtr` "/Game/Levels/MainMenu.MainMenu"))))