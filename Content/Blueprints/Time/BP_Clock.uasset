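; BP_Clock is the night's in-game clock, ending the night in a win once it reaches 6:00.
; Each Tick advances GameTime at 72x speed, so six hours pass in five real minutes, then calls WinGame once on BP_BaseNightGameState.
; It then splits the time into digits for three text displays.
; StartCountdown sets a Started flag, which counting never checks; earlier threshold branches are unconnected.
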(event `self.ReceiveBeginPlay`
  (bind _asbp_base_night_game_state (cast `/Game/Blueprints/Game/BP_BaseNightGameState` (`GameplayStatics.GetGameState`)))
  (set `self.GameState` _asbp_base_night_game_state))

(event `self.ReceiveTick`
  (params (DeltaSeconds :type "Float (single-precision)"))
  (`self.CountTime` DeltaSeconds)
  (`self.CheckTimeState`)
  (`self.UpdateText`))

(fn `CheckTimeState`
  (if (not (`self.GameEnded`))
    (`|ExecutionSequence`
      (:`then_1`)
      (:`then_2`)
      (:`then_3`)
      (:`then_4`
        (if (>= (`self.GameTime`) 21600.0)
          (`/Game/Blueprints/Game/BP_BaseNightGameState.WinGame` (`self.GameState`))
          (set `self.GameEnded` true))))))

(fn `CountTime`
  (params (DeltaTime :type "Float (double-precision)"))
  (set `self.GameTime` (+ (* DeltaTime 72.0) (`self.GameTime`))))

(fn `StartCountdown`
  (set `self.Started` true))

(fn `UpdateText`
  (locals (Hours :type Integer) (Minutes :type Integer) (MinutesFirst :type Integer) (MinutesSecond :type Integer) (MinutesReal :type Integer))
  (bind _minutes (`local.Minutes`))
  (bind _output_get (set `local.MinutesReal` (/ (`KismetMathLibrary.FTrunc` (`self.GameTime`)) 60)))
  (set `local.Hours` (/ _output_get 60))
  (set `local.Minutes` (- (`local.MinutesReal`) (* (`local.Hours`) 60)))
  (set `local.MinutesFirst` (/ _minutes 10))
  (set `local.MinutesSecond` (mod _minutes 10))
  (`TextRenderComponent.K2_SetText` (`self.HoursOnes`) (`KismetTextLibrary.Conv_IntToText` (`local.Hours`)))
  (`TextRenderComponent.K2_SetText` (`self.MinutesTens`) (`KismetTextLibrary.Conv_IntToText` (`local.MinutesFirst`) false true 1 1))
  (`TextRenderComponent.K2_SetText` (`self.MinutesOnes`) (`KismetTextLibrary.Conv_IntToText` (`local.MinutesSecond`))))

(fn `UserConstructionScript`)